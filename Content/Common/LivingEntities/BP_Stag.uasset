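; BP_Stag is a living-entity character with melee-style attack, movement and range functions, plus a health readout.
; Attack plays a montage and signals attack end on completion or interruption.
; Damage reports a damage event crediting BP_Liora, passing remaining health as the amount, then lowers BPCHealth through a DoOnce that resets after a short delay.
; Tick refreshes the health text; helper functions supply attack/defend radii and map speed states to walk speed.
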(event Custom|Attack
  (Animation|Montage|PlayMontage (Variables|Character|GetMesh) "/Game/Characters/Mannequins/Animations/Stag/AM_Stag_Attack.AM_Stag_Attack"
    (:OnCompleted
      _)
    (:OnInterrupted
      _))
  (Default|CallOnAttackEnd))

(event EventTick
  (params (DeltaSeconds :type Float%20%28single-precision%29))
  (bind _bpc_health (Variables|Default|GetBPC_Health))
  (Rendering|Components|TextRender|SetText (Variables|Default|GetTextRender) (Utilities|Text|ToText(String) (Utilities|String|Append (Utilities|String|ToString(Float) (Variables|/Game/Common/Components/BPC_Health.BPC_Health_C|GetcurrentHealth _bpc_health)) " / " (Utilities|String|ToString(Float) (Variables|/Game/Common/Components/BPC_Health.BPC_Health_C|GetmaxHealth _bpc_health))))))

(event EventDamage
  (params (damageAmount :type Float%20%28double-precision%29))
  (bind _bpc_health (Variables|Default|GetBPC_Health))
  (bind _returnvalue (Actor|GetActorOfClass "/Game/Common/LivingEntities/BP_Liora.BP_Liora_C"))
  (Class|AISenseDamage|ReportDamageEvent self _returnvalue (- (Variables|/Game/Common/Components/BPC_Health.BPC_Health_C|GetcurrentHealth _bpc_health) damageAmount) (Transformation|GetActorLocation) "0, 0, 0" "None")
  (Utilities|FlowControl|DoOnce false :!label _label
    (:Completed
      (Variables|/Game/Common/Components/BPC_Health.BPC_Health_C|SetcurrentHealth _bpc_health (- (Variables|/Game/Common/Components/BPC_Health.BPC_Health_C|GetcurrentHealth _bpc_health) damageAmount))
      (Utilities|FlowControl|Delay 0.2)
      (goto _label Reset))))

(event EventBeginPlay
  (bind _bpc_health (Variables|Default|GetBPC_Health))
  ;[1 1 1] Sets the health of the dummy (Accessed when placed in world)
  (bind _output_get (Variables|/Game/Common/Components/BPC_Health.BPC_Health_C|SetmaxHealth _bpc_health 1e+01))
  (Variables|/Game/Common/Components/BPC_Health.BPC_Health_C|SetcurrentHealth _bpc_health _output_get))

(fn ConstructionScript)

(fn GetIdealRange
  (return 1e+02 3.5e+02))

(fn SetMovementSpeed
  (params (Speed%20 :type E_MovementSpeed%20Enum :default "NewEnumerator0"))
  (bind _output_get (Variables|/Script/Engine.CharacterMovementComponent|SetMaxWalkSpeed (Variables|Character|GetCharacterMovement) (Utilities|Select :Index Speed%20 :NewEnumerator0 0.0 :NewEnumerator1 2.5e+02 :NewEnumerator2 7.5e+02 :NewEnumerator3 125.0)))
  (return _output_get))