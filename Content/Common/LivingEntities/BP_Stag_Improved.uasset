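; BP_Stag_Improved is an AI-controlled stag that fights the player (BP_Liora) and becomes pacified when its health runs out.
; Attack plays a montage, applies delayed damage to Liora, and signals OnAttackEnd when the montage ends.
; Damage reports to AI perception and lowers health behind a short DoOnce cooldown, removing Niagara and text on hits at zero health.
; Tick updates health text and pacifies through AIC_Stag; functions supply combat ranges and movement speeds.
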(event Custom|Attack
  (Animation|Montage|PlayMontage (Variables|Character|GetMesh) "/Game/Characters/Mannequins/Animations/Stag/AM_Stag_Attack.AM_Stag_Attack"
    (:then
      (Utilities|FlowControl|Delay 0.5)
      (Game|Damage|ApplyDamage (Variables|Default|GetAs%20BP%20Liora) 1e+01 0 0))
    (:OnCompleted
      (Default|CallOnAttackEnd :!label _label))
    (:OnInterrupted
      (goto _label))))

(event EventTick
  (params (DeltaSeconds :type Float%20%28single-precision%29))
  (bind _bpc_health (Variables|Default|GetBPC_Health))
  (Utilities|FlowControl|Sequence
    (:then_0
      (Rendering|Components|TextRender|SetText (Variables|Default|GetTextRender) (Utilities|Text|ToText(String) (Utilities|String|Append (Utilities|String|ToString(Float) (Variables|/Game/Common/Components/BPC_Health.BPC_Health_C|GetcurrentHealth _bpc_health)) " / " (Utilities|String|ToString(Float) (Variables|/Game/Common/Components/BPC_Health.BPC_Health_C|GetmaxHealth _bpc_health))))))
    (:then_1
      ;[1 1 1] Set State to Pacified
      (if (<= (Variables|/Game/Common/Components/BPC_Health.BPC_Health_C|GetcurrentHealth (Variables|Default|GetBPC_Health)) 0.0)
        (AI|Components|Blackboard|SetValueasBool (AI|GetBlackboard 0) (Utilities|Name|MakeLiteralName (Variables|Default|GetValue)) false)
        (bind _asaic_stag (Utilities|Casting|CastToAIC_Stag (AI|GetAIController self)))
        (Default|SetStatePacified _asaic_stag)))))

(event EventDamage
  (params (damageAmount :type Float%20%28double-precision%29))
  (bind _returnvalue (Transformation|GetActorLocation))
  (bind _bpc_health (Variables|Default|GetBPC_Health))
  (bind _returnvalue_2 (Actor|GetActorOfClass "/Game/Common/LivingEntities/BP_Liora.BP_Liora_C"))
  (Class|AISenseDamage|ReportDamageEvent self _returnvalue_2 (- (Variables|/Game/Common/Components/BPC_Health.BPC_Health_C|GetcurrentHealth _bpc_health) damageAmount) _returnvalue "0, 0, 0" "None")
  (Class|AISenseDamage|ReportDamageEvent self _returnvalue_2 damageAmount _returnvalue "0, 0, 0" "None")
  (if (> (Variables|/Game/Common/Components/BPC_Health.BPC_Health_C|GetcurrentHealth _bpc_health) 0.0)
    (Utilities|FlowControl|DoOnce false :!label _label
      (:Completed
        (Variables|/Game/Common/Components/BPC_Health.BPC_Health_C|SetcurrentHealth _bpc_health (- (Variables|/Game/Common/Components/BPC_Health.BPC_Health_C|GetcurrentHealth _bpc_health) damageAmount))
        (Utilities|FlowControl|Delay 0.2)
        (goto _label Reset)))
    (else
      ;[1 1 1] Destroy Niagara and Text Render
      (Components|DestroyComponent (Variables|Default|GetNiagara))
      (Components|DestroyComponent (Variables|Default|GetTextRender)))))

(event EventBeginPlay
  (bind _bpc_health (Variables|Default|GetBPC_Health))
  ;[1 1 1] Sets the health of the dummy (Accessed when placed in world)
  (Utilities|FlowControl|Sequence
    (:then_0
      (bind _output_get (Variables|/Game/Common/Components/BPC_Health.BPC_Health_C|SetmaxHealth _bpc_health 1e+01))
      (Variables|/Game/Common/Components/BPC_Health.BPC_Health_C|SetcurrentHealth _bpc_health _output_get))
    (:then_1
      (bind _asbp_liora (Utilities|Casting|CastToBP_Liora (Game|GetPlayerCharacter 0)))
      (Variables|Default|SetAs%20BP%20Liora _asbp_liora))))

(fn ConstructionScript)

(fn GetIdealRange
  (return 1e+02 3.5e+02))

(fn SetMovementSpeed
  (params (Speed%20 :type E_MovementSpeed%20Enum :default "NewEnumerator0"))
  (bind _output_get (Variables|/Script/Engine.CharacterMovementComponent|SetMaxWalkSpeed (Variables|Character|GetCharacterMovement) (Utilities|Select :Index Speed%20 :NewEnumerator0 0.0 :NewEnumerator1 2.5e+02 :NewEnumerator2 7.5e+02 :NewEnumerator3 125.0)))
  (return _output_get))