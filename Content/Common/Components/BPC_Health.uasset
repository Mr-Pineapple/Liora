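; BPC_Health is an actor component that tracks an entity's health and signals its death.
; BeginPlay sets failsafe health values, while SetHealthComponent sets max and current health from a supplied value.
; ApplyDamage subtracts damage behind a DoOnce that resets after a short delay, ignoring hits in that window.
; After that delay, NoHealth calls the death dispatcher if health is near or below zero.
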(event Custom|ApplyDamage
  (params (damageAmount :type Float%20%28double-precision%29))
  ;[1 1 1] Applys given damage to entity - implement from the damage message
  (Utilities|FlowControl|DoOnce false :!label _label
    (:Completed
      (Variables|Default|SetcurrentHealth (- (Variables|Default|GetcurrentHealth) damageAmount))
      (Utilities|FlowControl|Delay 0.2)
      (CallFunction|NoHealth)
      (goto _label Reset))))

(event Custom|SetHealthComponent
  (params (healthValue :type Float%20%28double-precision%29))
  ;[1 1 1] Set the health of the entity when initializing
  (bind _output_get (Variables|Default|SetmaxHealth healthValue))
  (Variables|Default|SetcurrentHealth _output_get))

(event Custom|NoHealth
  (if (<= (Variables|Default|GetcurrentHealth) 0.1)
    (Default|CallDeathDispatch)))

(event EventBeginPlay
  ;[1 0 0] Used as a failsafe to set health values
  (bind _output_get (Variables|Default|SetmaxHealth 5e+01))
  (Variables|Default|SetcurrentHealth _output_get))