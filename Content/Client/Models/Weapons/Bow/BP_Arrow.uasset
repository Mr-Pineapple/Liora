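; BP_Arrow is a bow projectile that deals damage and sticks into what it hits.
; Fire enables collision and adds a projectile movement component at runtime, with draw strength scaling speed and gravity, plus sound, trail and timeline-driven spin.
; On overlapping anything but its instigator, it stops, attaches to the hit component or bone, then sends BPI_HealthSystem damage or plays impact effects and pushes physics objects.
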(event OnComponentBeginOverlap(Collision)
  (params (OverlappedComponent :type Primitive%20Component%20Object%20Reference) (OtherActor :type Actor%20Object%20Reference) (OtherComp :type Primitive%20Component%20Object%20Reference) (OtherBodyIndex :type Integer) (bFromSweep :type Boolean) (SweepResult :type Hit%20Result%20Structure%20%28by%20ref%29))
  (bind (_bblockinghit _binitialoverlap _time _distance _location _impactpoint _normal _impactnormal _physmat _hitactor _hitcomponent _hitbonename _bonename _hititem _elementindex _faceindex _tracestart _traceend) (Collision|BreakHitResult SweepResult))
  (if (not (== (Game|GetInstigator) OtherActor))
    (bind _projectilemovementcomponent (Variables|Default|GetProjectileMovementComponent)
      (:then
        (Components|DestroyComponent _projectilemovementcomponent))
      (:else
        _))
    (Audio|Components|Audio|Stop (Variables|Default|GetSpinArrowTimeline))
    (Collision|SetCollisionEnabled (Variables|Default|GetCollision) "NoCollision")
    (Transformation|SetActorLocation _impactpoint false false)
    (Transformation|AttachComponentToComponent OtherComp _hitbonename "KeepWorld" "KeepWorld" "KeepWorld" true)
    (if (Utilities|DoesObjectImplementInterface _hitactor "/Game/Common/Components/BPI_HealthSystem.BPI_HealthSystem_C")
      (Class|BPIHealthSystem|Damage(Message) _hitactor 3.0)
      (else
        (Audio|PlaySoundatLocation (Variables|Default|GetImpactSound) _impactpoint "0, 0, 0" 1.0 1.0 0.0 0 0 0 0)
        (Effects|SpawnEmitteratLocation 0 _impactpoint)
        (if (Physics|IsSimulatingPhysics OtherComp "None")
          (Physics|AddImpulse OtherComp (* (Math|Vector|GetUnitDirection(Vector) _tracestart _traceend) (Math|Vector|VectorLength (Transformation|GetVelocity))) "None" true))
        (Utilities|FlowControl|Delay 1.0)
        (bind _traileffectref (Variables|Default|GetTrailEffectRef)
          (:then
            (Components|DestroyComponent _traileffectref))
          (:else))))))

(event Custom|Fire
  (params (Direction :type Vector) (Strength :type Float%20%28double-precision%29))
  (Collision|SetCollisionEnabled (Variables|Default|GetCollision) "QueryOnly")
  (bind _returnvalue (AddComponent|AddProjectileMovementComponent))
  (bind _output_get (Variables|Default|SetProjectileMovementComponent _returnvalue))
  (Variables|/Script/Engine.MovementComponent|SetVelocity _output_get (* Direction (Math|Float|Lerp (Variables|Default|GetMinArrowSpeed) (Variables|Default|GetMaxArrowSpeed) Strength)))
  (Variables|/Script/Engine.ProjectileMovementComponent|SetProjectileGravityScale _returnvalue (Math|Float|Lerp (Variables|Default|GetMaxArrowGravity) (Variables|Default|GetMinArrowGravity) Strength))
  (Audio|PlaySoundatLocation (Variables|Default|GetArrowWhooshSound) (Transformation|GetActorLocation) "0, 0, 0" 1.0 1.0 0.0 0 0 0 0)
  (bind _returnvalue_2 (Niagara|SpawnSystemAttached (Variables|Default|GetTrailEffectTemplate) (Variables|Default|GetParticleAttachPoint) "None" "0, 0, 0" "0, 0, 0" "KeepRelativeOffset" false))
  (Variables|Default|SetTrailEffectRef _returnvalue_2)
  (Actor|SetLifeSpan 5.0)
  (CallFunction|SpinStart))

(event Custom|SpinStart
  (bind _xrotation (Timeline|SpinArrowTimeline Play)
    (:Update
      (Transformation|SetRelativeRotation (Variables|Default|GetStaticMesh) (Math|Rotator|MakeRotator _xrotation 0.0 0.0) false false))))

(event EventBeginPlay
  (Collision|SetCollisionEnabled (Variables|Default|GetCollision) "NoCollision"))

(fn ConstructionScript)