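; Actor component that gives a Character bow combat: equipping a bow, aiming, drawing and firing arrows.
; Aiming switches the character to controller-facing rotation and attaches an arrow, while drawing runs a looping timer that broadcasts draw time.
; Release scales strength by draw time and aims the arrow at a camera trace point, correcting for socket offset.
; After the fire montage, aiming re-arms and any queued draw resumes.
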(event Custom|AimBegin
  (bind _characterref (Variables|Default|GetCharacterRef))
  (bind _charactermovement (Variables|/Script/Engine.Character|GetCharacterMovement _characterref))
  ;[1 1 1] Aiming
  (Variables|Default|SetIsAiming true)
  (Variables|/Game/Client/Models/Weapons/Bow/BP_Bow.BP_Bow_C|SetDrawState (Variables|Default|GetEquippedBow) "NewEnumerator1")
  (Variables|/Script/Engine.CharacterMovementComponent|SetbOrientRotationToMovement _charactermovement false)
  (Variables|/Script/Engine.CharacterMovementComponent|SetbUseControllerDesiredRotation _charactermovement true)
  (Variables|/Script/Engine.CharacterMovementComponent|SetRotationRate _charactermovement "0.000000,1000.000000,0.000000")
  (CallFunction|SpawnArrow)
  (Default|CallOnAimStart))

(event Custom|Initialize
  (params (BowClass :type BP%20Bow%20Class%20Reference) (BowSocketName :type Name) (ArrowSocketName :type Name) (FireArrowMontage :type Anim%20Montage%20Object%20Reference))
  (Variables|Default|SetBowClass BowClass)
  (Variables|Default|SetBowSocketName BowSocketName)
  (Variables|Default|SetArrowSocketName ArrowSocketName)
  (Variables|Default|SetFireArrowMontage FireArrowMontage)
  (CallFunction|EquipBow))

(event Custom|DrawBegin
  ;[1 1 1] Drawing Bow
  (Utilities|CanDrawBow
    (:Yes
      (Variables|Default|SetIsDrawingBow true)
      (Variables|/Game/Client/Models/Weapons/Bow/BP_Bow.BP_Bow_C|SetDrawState (Variables|Default|GetEquippedBow) "NewEnumerator2")
      (bind _returnvalue (Audio|SpawnSound2D "/Game/Client/Audio/Cues/Cue_Arrow_Draw.Cue_Arrow_Draw" 1.0 1.0 0.0 0))
      (Variables|Default|SetDrawBowSound _returnvalue)
      (bind _returnvalue_2 (Utilities|Time|SetTimerbyEvent (delegate Custom|IncrementDrawBowTime) (Variables|Default|GetDrawUpdateInterval) true))
      (Variables|Default|SetIncrementDrawBowTimeHandler _returnvalue_2))
    (:No
      (Variables|Default|SetIsWaitingToDrawBow true))))

(event Custom|DrawEnd
  ;[1 1 1] Drawing Bow
  (Variables|Default|SetIsDrawingBow false)
  (Variables|/Game/Client/Models/Weapons/Bow/BP_Bow.BP_Bow_C|SetDrawState (Variables|Default|GetEquippedBow) "NewEnumerator1")
  (Variables|Default|SetIsWaitingToDrawBow false)
  (Utilities|Time|ClearandInvalidateTimerbyHandle (Variables|Default|GetIncrementDrawBowTimeHandler))
  (Variables|Default|SetDrawTime 0.0)
  (bind _drawbowsound (Variables|Default|GetDrawBowSound)
    (:then
      (Audio|Components|Audio|Stop _drawbowsound))
    (:else
      _))
  (Default|CallOnDrawEnd))

(event Custom|FireArrowBegin
  ;[1 1 1] Firing Arrow
  (Utilities|CanFireArrow
    (:Yes
      (Variables|Default|SetIsFiringArrow true)
      (CallFunction|FireAimedArrow)
      (CallFunction|DrawEnd)
      (Animation|Montage|PlayMontage (Variables|/Game/Client/Models/Weapons/Bow/BP_Bow.BP_Bow_C|GetBowSkeletalMesh (Variables|Default|GetEquippedBow)) (Variables|/Game/Client/Models/Weapons/Bow/BP_Bow.BP_Bow_C|GetBowReleaseMontage (Variables|Default|GetEquippedBow))
        (:then
          (Animation|Montage|PlayMontage (Variables|/Script/Engine.Character|GetMesh (Variables|Default|GetCharacterRef)) (Variables|Default|GetFireArrowMontage)
            (:OnCompleted
              _)
            (:OnInterrupted
              _))
          (CallFunction|FireArrowEnd))))))

(event Custom|FireArrowEnd
  ;[1 1 1] Firing Arrow
  (Variables|Default|SetIsFiringArrow false)
  (if (Variables|Default|GetIsAiming)
    (CallFunction|AimBegin)
    (if (Variables|Default|GetIsWaitingToDrawBow)
      (CallFunction|DrawBegin)
      (Variables|Default|SetIsWaitingToDrawBow false))))

(event Custom|IncrementDrawBowTime
  ;[1 1 1] Drawing Bow
  (bind _output_get (Variables|Default|SetDrawTime (+ (Variables|Default|GetDrawTime) (Variables|Default|GetDrawUpdateInterval))))
  (Default|CallOnDrawUpdate _output_get (Variables|/Game/Client/Models/Weapons/Bow/BP_Bow.BP_Bow_C|GetMaxDrawTime (Variables|Default|GetEquippedBow))))

(event Custom|AimEnd
  (bind _characterref (Variables|Default|GetCharacterRef))
  (bind _charactermovement (Variables|/Script/Engine.Character|GetCharacterMovement _characterref))
  ;[1 1 1] Aiming
  (Variables|Default|SetIsAiming false)
  (CallFunction|DrawEnd)
  (Variables|/Game/Client/Models/Weapons/Bow/BP_Bow.BP_Bow_C|SetDrawState (Variables|Default|GetEquippedBow) "NewEnumerator0")
  (Variables|/Script/Engine.CharacterMovementComponent|SetbOrientRotationToMovement _charactermovement true)
  (Variables|/Script/Engine.CharacterMovementComponent|SetbUseControllerDesiredRotation _charactermovement false)
  (Variables|/Script/Engine.CharacterMovementComponent|SetRotationRate _charactermovement "0.000000,360.000000,0.000000")
  (CallFunction|DestroyAimedArrow)
  (Default|CallOnAimEnd))

(event EventBeginPlay
  (bind _ascharacter (Utilities|Casting|CastToCharacter (Components|GetOwner)))
  (Variables|Default|SetCharacterRef _ascharacter))

(fn EquipBow
  (Variables|Default|GetEquippedBow
    (:then)
    (:else
      (bind _returnvalue (Game|SpawnActorfromClass (Variables|Default|GetBowClass) (Math|Transform|MakeTransform "0, 0, 0" "0, 0, 0" "1.000000,1.000000,1.000000") "Undefined" "MultiplyWithRoot" 0 0))
      (bind _output_get (Variables|Default|SetEquippedBow _returnvalue))
      (Transformation|AttachComponentToComponent _output_get (Variables|/Script/Engine.Character|GetMesh (Variables|Default|GetCharacterRef)) (Variables|Default|GetBowSocketName) "SnapToTarget" "SnapToTarget" "SnapToTarget" true))))

(fn SpawnArrow
  (Variables|Default|GetAimedArrow
    (:then)
    (:else
      (bind _returnvalue (Game|SpawnActorfromClass "/Game/Client/Models/Weapons/Bow/BP_Arrow.BP_Arrow_C" (Math|Transform|MakeTransform "0, 0, 0" "0, 0, 0" "1.000000,1.000000,1.000000") "Undefined" "MultiplyWithRoot" 0 (Variables|Default|GetCharacterRef)))
      (bind _output_get (Variables|Default|SetAimedArrow _returnvalue))
      (Transformation|AttachComponentToComponent _output_get (Variables|/Script/Engine.Character|GetMesh (Variables|Default|GetCharacterRef)) (Variables|Default|GetArrowSocketName) "SnapToTarget" "SnapToTarget" "SnapToTarget" true))))

(fn DestroyAimedArrow
  (bind _aimedarrow (Variables|Default|GetAimedArrow)
    (:then
      (Actor|DestroyActor _aimedarrow))
    (:else)))

(fn FireAimedArrow
  (bind _aimedarrow (Variables|Default|GetAimedArrow)
    (:then
      (Transformation|DetachFromActor _aimedarrow "KeepWorld" "KeepWorld" "KeepWorld")
      (bind _direction (CallFunction|CalculateArrowDirection))
      (Default|Fire _aimedarrow _direction (Math|Float|Clamp(Float) (Math|Float|NormalizetoRange (Variables|Default|GetDrawTime) 0.0 (Variables|/Game/Client/Models/Weapons/Bow/BP_Bow.BP_Bow_C|GetMaxDrawTime (Variables|Default|GetEquippedBow)))))
      (Variables|Default|SetAimedArrow 0))
    (:else)))

(fn CalculateArrowDirection
  (bind _characterref (Variables|Default|GetCharacterRef))
  (bind _returnvalue (Actor|GetComponentbyClass _characterref "/Script/Engine.CameraComponent"))
  (bind _returnvalue_2 (Transformation|GetWorldLocation _returnvalue))
  (bind _returnvalue_3 (Math|Vector|GetForwardVector _returnvalue))
  (Utilities|IsValid _returnvalue
    (:Is%20Valid
      (bind (_outhit _returnvalue_4) (Collision|LineTraceByChannel (+ _returnvalue_2 (* _returnvalue_3 3e+02)) (+ _returnvalue_2 (* _returnvalue_3 1e+04)) "TraceTypeQuery1" false 0 "None"))
      (bind _aimedarrow (Variables|Default|GetAimedArrow)
        (:then
          (return (Math|Vector|GetUnitDirection(Vector) (Transformation|GetActorLocation _aimedarrow) (Math|Vector|SelectVector (.Location (Collision|BreakHitResult _outhit)) (.TraceEnd (Collision|BreakHitResult _outhit)) _returnvalue_4))))
        (:else)))))