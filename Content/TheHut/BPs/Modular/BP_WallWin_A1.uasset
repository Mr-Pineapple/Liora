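; Modular wooden wall piece for TheHut, with optional window pillars, window doors and a second interior wall, built in the construction script.
; It picks random meshes for the main wall, pillars and window doors, placing added components from transform arrays with a yaw offset for door opening.
; Window doors require pillars to be enabled, while interior walls always use the first wall mesh and skip the cull distance and forced LOD settings.
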(event EventBeginPlay)

(event Collision|EventActorBeginOverlap
  (params (OtherActor :type Actor%20Object%20Reference)))

(event EventTick
  (params (DeltaSeconds :type Float%20%28single-precision%29)))

(fn ConstructionScript
  (bind _sm_wallwood_a1 (Variables|Default|GetSM_WallWood_A1))
  (Variables|Mesh|SetUpdate false)
  (if (Variables|Mesh|GetTwo%20Wall)
    (Utilities|FlowControl|Sequence
      (:then_0
        (Components|StaticMesh|SetStaticMesh _sm_wallwood_a1 (Utilities|Array|Get(acopy) (Variables|Mesh|GetWall%20-%20New%20SMs) (Math|Random|RandomIntegerinRange (Variables|Mesh|GetWall%20-%20Random%20Min) (Variables|Mesh|GetWall%20-%20Random%20Max))) :!label _label)
        (Class|PrimitiveComponent|SetCullDistance _sm_wallwood_a1 (Variables|Mesh|GetCull%20Distance))
        (Rendering|LOD|SetForcedLodModel _sm_wallwood_a1 (Variables|Mesh|GetForce%20LOD%20Models))
        (if (Variables|Mesh|GetHave%20Pillar%20For%20Windows)
          (Utilities|FlowControl|Sequence
            (:then_0
              (for _array_element (Variables|Mesh|GetPillars%20Location)
                (bind _returnvalue (AddComponent|AddStaticMeshComponent false _array_element))
                (Components|StaticMesh|SetStaticMesh _returnvalue (Utilities|Array|Get(acopy) (Variables|Mesh|GetPillar%20-%20New%20SMs) (Math|Random|RandomIntegerinRange 0 1)))
                (Class|PrimitiveComponent|SetCullDistance _returnvalue (Variables|Mesh|GetCull%20Distance))
                (Rendering|LOD|SetForcedLodModel _returnvalue (Variables|Mesh|GetForce%20LOD%20Models))))
            (:then_1
              (if (Variables|Windows/Door|GetHave%20Windows/Door)
                (for _array_element_2 (Variables|Windows/Door|GetWin/Door%20Location)
                  (bind _returnvalue_2 (AddComponent|AddStaticMeshComponent false (Math|Transform|MakeTransform (.Location (Math|Transform|BreakTransform _array_element_2)) (Math|Rotator|MakeRotator (.roll (.Rotation (Math|Transform|BreakTransform _array_element_2))) (.pitch (.Rotation (Math|Transform|BreakTransform _array_element_2))) (+ (.yaw (.Rotation (Math|Transform|BreakTransform _array_element_2))) (Variables|Win/DoorOpen|GetOpen%20Win/Door))) (.Scale (Math|Transform|BreakTransform _array_element_2)))))
                  (Components|StaticMesh|SetStaticMesh _returnvalue_2 (Utilities|Array|Get(acopy) (Variables|Windows/Door|GetWindows/Door%20-%20New%20SMs) (Math|Random|RandomIntegerinRange (Variables|Windows/Door|GetWin/Door%20-%20Random%20Min) (Variables|Windows/Door|GetWin/Door%20-%20Random%20Max))))
                  (Class|PrimitiveComponent|SetCullDistance _returnvalue_2 (Variables|Mesh|GetCull%20Distance))
                  (Rendering|LOD|SetForcedLodModel _returnvalue_2 (Variables|Mesh|GetForce%20LOD%20Models))))))))
      (:then_1
        (for _array_element_3 (Variables|Mesh|GetWall%20Interior)
          (bind _returnvalue_3 (AddComponent|AddStaticMeshComponent false _array_element_3))
          (Components|StaticMesh|SetStaticMesh _returnvalue_3 (Utilities|Array|Get(acopy) (Variables|Mesh|GetWall%20-%20New%20SMs) (Math|Random|RandomIntegerinRange 0 0))))))
    (else
      (goto _label))))