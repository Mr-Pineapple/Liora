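; BP_Wall_A1 is a modular wall piece for TheHut that assembles randomized wall and pillar meshes in the Construction Script, with no active event logic.
; It picks the main wall mesh from an index range, optionally spawns random pillars at listed transforms, and applies cull distance and forced LOD to both.
; TwoWalls adds interior wall meshes without those settings.
; Randomization is unseeded, and the Update flag resets on each construction run.
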(event EventBeginPlay)

(event Collision|EventActorBeginOverlap
  (params (OtherActor :type Actor%20Object%20Reference)))

(event EventTick
  (params (DeltaSeconds :type Float%20%28single-precision%29)))

(fn ConstructionScript
  (bind _sm_wallwood_a1 (Variables|Default|GetSM_WallWood_A1))
  (Variables|Wall|SetUpdate false)
  (if (Variables|Wall|GetTwo%20Walls)
    (Utilities|FlowControl|Sequence
      (:then_0
        (Components|StaticMesh|SetStaticMesh _sm_wallwood_a1 (Utilities|Array|Get(acopy) (Variables|Wall|GetWall%20-%20New%20SMs) (Math|Random|RandomIntegerinRange (Variables|Wall|GetWall%20-%20Random%20Min) (Variables|Wall|GetWall%20-%20Random%20Max))) :!label _label)
        (Class|PrimitiveComponent|SetCullDistance _sm_wallwood_a1 (Variables|Wall|GetCull%20Distance))
        (Rendering|LOD|SetForcedLodModel _sm_wallwood_a1 (Variables|Wall|GetForce%20LOD%20Models))
        (if (Variables|Pillar|GetHave%20Pillar)
          (for _array_element (Variables|Pillar|GetPillars%20Location)
            (bind _returnvalue (AddComponent|AddStaticMeshComponent false _array_element))
            (Components|StaticMesh|SetStaticMesh _returnvalue (Utilities|Array|Get(acopy) (Variables|Pillar|GetPillar%20-%20New%20SMs) (Math|Random|RandomIntegerinRange (Variables|Pillar|GetPillar%20-%20Random%20Min) (Variables|Pillar|GetPillar%20-%20Random%20Max))))
            (Class|PrimitiveComponent|SetCullDistance _returnvalue (Variables|Wall|GetCull%20Distance))
            (Rendering|LOD|SetForcedLodModel _returnvalue (Variables|Wall|GetForce%20LOD%20Models)))))
      (:then_1
        (for _array_element_2 (Variables|Wall|GetWall%20Interior)
          (bind _returnvalue_2 (AddComponent|AddStaticMeshComponent false _array_element_2))
          (Components|StaticMesh|SetStaticMesh _returnvalue_2 (Utilities|Array|Get(acopy) (Variables|Wall|GetWall%20-%20New%20SMs) (Math|Random|RandomIntegerinRange (Variables|Wall|GetWall%20-%20Random%20Min) (Variables|Wall|GetWall%20-%20Random%20Max)))))))
    (else
      (goto _label))))