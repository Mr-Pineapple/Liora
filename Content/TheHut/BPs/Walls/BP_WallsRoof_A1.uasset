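; BP_WallsRoof_A1 is a roof wall piece for the hut environment, built from ten plank mesh components with randomized meshes.
; The Construction Script gives each plank a random mesh from the first thirteen entries of the PlanksSMs array.
; The roll is unseeded, so each construction rerun reshuffles the look, and an Update flag resets to false each time.
; The event graph holds no active logic.
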(event EventBeginPlay)

(event Collision|EventActorBeginOverlap
  (params (OtherActor :type Actor%20Object%20Reference)))

(event EventTick
  (params (DeltaSeconds :type Float%20%28single-precision%29)))

(fn ConstructionScript
  (Variables|Default|SetUpdate false)
  (for _array_element (Utilities|Array|MakeArray (Variables|Default|GetSM_Plank_A6) (Variables|Default|GetSM_Plank_A2) (Variables|Default|GetSM_Plank_A3) (Variables|Default|GetSM_Plank_A4) (Variables|Default|GetSM_Plank_A5) (Variables|Default|GetSM_Plank_A1) (Variables|Default|GetSM_Plank_A7) (Variables|Default|GetSM_Plank_A8) (Variables|Default|GetSM_Plank_A9) (Variables|Default|GetSM_Plank_A10))
    (Components|StaticMesh|SetStaticMesh _array_element (Utilities|Array|Get(acopy) (Variables|Default|GetPlanks%20SMs) (Math|Random|RandomIntegerinRange 0 12)))))