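; BP_Hut_E1 is a configurable modular hut prop, assembled entirely in the Construction Script with no active event logic.
; Option flags destroy unused mesh components to choose ceiling, stairs, outer roof and one of two roof tops.
; It applies a forced LOD and cull distance to the meshes.
; A SetColor helper creates dynamic material instances per slot, tinting "Base Color" from two main colors and a ceiling color.
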(event EventBeginPlay)

(event Collision|EventActorBeginOverlap
  (params (OtherActor :type Actor%20Object%20Reference)))

(event EventTick
  (params (DeltaSeconds :type Float%20%28single-precision%29)))

(fn ConstructionScript
  (bind _sm_hute_ceilingnotstairs (Variables|Default|GetSM_HutE_CeilingNotStairs))
  (bind _color_b (Variables|Color|GetColor%20B))
  (bind _sm_hute (Variables|Default|GetSM_HutE))
  (bind _sm_hute_stairs (Variables|Default|GetSM_HutE_Stairs))
  (bind _sm_hute_roof (Variables|Default|GetSM_HutE_Roof))
  (bind _sm_hute_rooftopa (Variables|Default|GetSM_HutE_RoofTopA))
  (bind _sm_hute_rooftopb (Variables|Default|GetSM_HutE_RoofTopB))
  (bind _sm_hute_roof_2 (Variables|Default|GetSM_HutE_Roof))
  (bind _color_a (Variables|Color|GetColor%20A))
  (bind _color_b_2 (Variables|Color|GetColor%20B))
  (Utilities|FlowControl|Sequence
    (:then_0
      (if (Variables|Edit|GetCeiling)
        _
        (else
          (Components|DestroyComponent (Variables|Default|GetSM_HutE_Ceiling))))
      (if (Variables|Edit|GetStairs)
        (Components|DestroyComponent (Variables|Default|GetSM_HutE_CeilingNotStairs))
        (else
          (Components|DestroyComponent (Variables|Default|GetSM_HutE_Stairs))))
      (Rendering|LOD|SetForcedLodModel _sm_hute_roof_2 (Variables|Edit|GetForce%20LOD))
      ;[1 0 0] If it is less than 19K, it will be discarded before LOD 3 (last LOD). 30K will have good use in open world games.
      (Class|PrimitiveComponent|SetCullDistance _sm_hute_roof_2 (Variables|Edit|GetCull%20Distance)))
    (:then_1
      (if (Variables|Edit|GetOutRoof)
        _
        (else
          (Components|DestroyComponent (Variables|Default|GetSM_HutE_Ranch))))
      (if (Variables|Edit|GetRoof%20A/B)
        (Components|DestroyComponent (Variables|Default|GetSM_HutE_RoofTopB))
        (else
          (Components|DestroyComponent (Variables|Default|GetSM_HutE_RoofTopA)))))
    (:then_2
      (Utilities|FlowControl|Sequence
        (:then_0
          ;[1 1 1] Hut Color
          (CallFunction|SetColor _sm_hute 0 _color_a)
          (CallFunction|SetColor _sm_hute 1 _color_b_2)
          (CallFunction|SetColor _sm_hute 2 _color_b_2)
          (CallFunction|SetColor _sm_hute 3 _color_a)
          (CallFunction|SetColor _sm_hute 4 _color_b_2)
          (CallFunction|SetColor _sm_hute 5 _color_a)
          (CallFunction|SetColor _sm_hute 6 _color_a))
        (:then_1
          (CallFunction|SetColor _sm_hute_stairs 0 (Variables|Color|GetColor%20B))
          (CallFunction|SetColor _sm_hute_stairs 1 (Variables|Color|GetColor%20A))
          (CallFunction|SetColor (Variables|Default|GetSM_HutE_Ceiling) 0 (Variables|Color|GetCeiling%20Color))
          (CallFunction|SetColor (Variables|Default|GetSM_HutE_Ranch) 1 (Variables|Color|GetColor%20A))
          (CallFunction|SetColor _sm_hute_ceilingnotstairs 0 (Variables|Color|GetCeiling%20Color))
          (CallFunction|SetColor _sm_hute_ceilingnotstairs 1 (Variables|Color|GetColor%20A)))
        (:then_2
          (CallFunction|SetColor _sm_hute_roof 0 _color_b)
          (CallFunction|SetColor _sm_hute_roof 1 _color_b)
          (CallFunction|SetColor _sm_hute_roof 2 (Variables|Color|GetColor%20A))
          (CallFunction|SetColor _sm_hute_rooftopa 0 (Variables|Color|GetColor%20B))
          (CallFunction|SetColor _sm_hute_rooftopa 1 (Variables|Color|GetColor%20A))
          (CallFunction|SetColor _sm_hute_rooftopb 0 (Variables|Color|GetColor%20B))
          (CallFunction|SetColor _sm_hute_rooftopb 1 (Variables|Color|GetColor%20A)))))))

(fn SetColor
  (params (SM%20Target :type Primitive%20Component%20Object%20Reference) (Index%20MAT :type Integer) (Color :type Linear%20Color%20Structure))
  (bind _returnvalue (Rendering|Material|CreateDynamicMaterialInstance SM%20Target Index%20MAT 0 "None" :!class /Script/Engine.PrimitiveComponent))
  (Rendering|Material|SetVectorParameterValue _returnvalue "Base Color" Color :!class /Script/Engine.MaterialInstanceDynamic))