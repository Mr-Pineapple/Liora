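; BP_MountainHut_A1 is a configurable modular mountain hut prop, built entirely in its Construction Script.
; It offsets the main hut mesh, removes fence and bridge components by toggle, and applies forced LOD and cull distance only when the bridge is off.
; Dynamic material instances tint each mesh slot from structure, roof and two stair colors, with the stair colors shared by fences, pillars, planks and floor.
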(event EventBeginPlay)

(event Collision|EventActorBeginOverlap
  (params (OtherActor :type Actor%20Object%20Reference)))

(event EventTick
  (params (DeltaSeconds :type Float%20%28single-precision%29)))

(fn ConstructionScript
  (bind _sm_mhut_stairs (Variables|Default|GetSM_MHut_Stairs))
  (bind _stairs_color_a (Variables|Color|GetStairs%20Color%20A))
  (bind _stairs_color_b (Variables|Color|GetStairs%20Color%20B))
  (bind _sm_mhut_bridgefence (Variables|Default|GetSM_MHut_BridgeFence))
  (bind _sm_mhut_a3 (Variables|Default|GetSM_MHut_A3))
  (bind _sm_mhut_a1 (Variables|Default|GetSM_MHut_A1))
  (bind _sm_mhut_a2 (Variables|Default|GetSM_MHut_A2))
  (bind _sm_mhut_stairs_2 (Variables|Default|GetSM_MHut_Stairs))
  (bind _sm_mhut_a1_2 (Variables|Default|GetSM_MHut_A1))
  (Utilities|FlowControl|Sequence
    (:then_0
      ;[1 1 1] Location Hut
      (Transformation|SetRelativeLocation (Variables|Default|GetSM_MHut_A1) (Math|Vector|MakeVector (Variables|Edit|GetLocation%20X) 0.0 0.0) false false)
      ;[1 1 1] Have Fences?
      (if (Variables|Edit|GetFences?)
        _
        (else
          (Components|DestroyComponent (Variables|Default|GetSM_MHut_A3))))
      ;[1 1 1] Have Bridge?
      (if (not (Variables|Edit|GetBridge?))
        (Components|DestroyComponent (Variables|Default|GetSM_MHut_BridgeFloor))
        ;[1 1 1] Optimization
        (Rendering|LOD|SetForcedLodModel _sm_mhut_stairs_2 (Variables|Edit|GetForce%20LOD))
        ;;[1 0 0] If it is less than 19K, it will be discarded before LOD 3 (last LOD). 30K will have good use in open world games.
        (Class|PrimitiveComponent|SetCullDistance _sm_mhut_stairs_2 (Variables|Edit|GetCull%20Distance))))
    (:then_1
      ;[1 1 1] Structures Color
      (bind _returnvalue (Rendering|Material|CreateDynamicMaterialInstance (Variables|Default|GetSM_MHut_Structures) 0 0 "None" :!class /Script/Engine.PrimitiveComponent))
      (Rendering|Material|SetVectorParameterValue _returnvalue "Base Color" (Variables|Color|GetStructures%20Color) :!class /Script/Engine.MaterialInstanceDynamic)
      ;[1 1 1] Stairs Color
      (bind _returnvalue_2 (Rendering|Material|CreateDynamicMaterialInstance _sm_mhut_stairs 0 0 "None" :!class /Script/Engine.PrimitiveComponent))
      (Rendering|Material|SetVectorParameterValue _returnvalue_2 "Base Color" _stairs_color_b :!class /Script/Engine.MaterialInstanceDynamic)
      (bind _returnvalue_3 (Rendering|Material|CreateDynamicMaterialInstance _sm_mhut_stairs 1 0 "None" :!class /Script/Engine.PrimitiveComponent))
      (Rendering|Material|SetVectorParameterValue _returnvalue_3 "Base Color" _stairs_color_a :!class /Script/Engine.MaterialInstanceDynamic)
      (bind _returnvalue_4 (Rendering|Material|CreateDynamicMaterialInstance _sm_mhut_stairs 2 0 "None" :!class /Script/Engine.PrimitiveComponent))
      (Rendering|Material|SetVectorParameterValue _returnvalue_4 "Base Color" _stairs_color_b :!class /Script/Engine.MaterialInstanceDynamic)
      (bind _returnvalue_5 (Rendering|Material|CreateDynamicMaterialInstance _sm_mhut_stairs 3 0 "None" :!class /Script/Engine.PrimitiveComponent))
      (Rendering|Material|SetVectorParameterValue _returnvalue_5 "Base Color" _stairs_color_a :!class /Script/Engine.MaterialInstanceDynamic)
      ;[1 1 1] Fences Color
      (bind _returnvalue_6 (Rendering|Material|CreateDynamicMaterialInstance _sm_mhut_bridgefence 0 0 "None" :!class /Script/Engine.PrimitiveComponent))
      (Rendering|Material|SetVectorParameterValue _returnvalue_6 "Base Color" (Variables|Color|GetStairs%20Color%20B) :!class /Script/Engine.MaterialInstanceDynamic)
      (bind _returnvalue_7 (Rendering|Material|CreateDynamicMaterialInstance _sm_mhut_bridgefence 1 0 "None" :!class /Script/Engine.PrimitiveComponent))
      (Rendering|Material|SetVectorParameterValue _returnvalue_7 "Base Color" (Variables|Color|GetStairs%20Color%20A) :!class /Script/Engine.MaterialInstanceDynamic)
      (bind _returnvalue_8 (Rendering|Material|CreateDynamicMaterialInstance _sm_mhut_a3 0 0 "None" :!class /Script/Engine.PrimitiveComponent))
      (Rendering|Material|SetVectorParameterValue _returnvalue_8 "Base Color" (Variables|Color|GetStairs%20Color%20A) :!class /Script/Engine.MaterialInstanceDynamic)
      (bind _returnvalue_9 (Rendering|Material|CreateDynamicMaterialInstance _sm_mhut_a3 1 0 "None" :!class /Script/Engine.PrimitiveComponent))
      (Rendering|Material|SetVectorParameterValue _returnvalue_9 "Base Color" (Variables|Color|GetStairs%20Color%20B) :!class /Script/Engine.MaterialInstanceDynamic)
      ;[1 1 1] Hut Color
      (Utilities|FlowControl|Sequence
        (:then_0
          (Utilities|FlowControl|Sequence
            (:then_0
              ;;[1 1 1] Pillars Color
              (bind _returnvalue_10 (Rendering|Material|CreateDynamicMaterialInstance _sm_mhut_a1_2 0 0 "None" :!class /Script/Engine.PrimitiveComponent)))
            (:then_1
              (bind _returnvalue_11 (Rendering|Material|CreateDynamicMaterialInstance _sm_mhut_a1_2 6 0 "None" :!class /Script/Engine.PrimitiveComponent)))
            (:then_2
              (bind _returnvalue_12 (Rendering|Material|CreateDynamicMaterialInstance _sm_mhut_a1_2 7 0 "None" :!class /Script/Engine.PrimitiveComponent))))
          (Rendering|Material|SetVectorParameterValue _returnvalue_10 "Base Color" (Variables|Color|GetStairs%20Color%20A) :!class /Script/Engine.MaterialInstanceDynamic))
        (:then_1
          (Utilities|FlowControl|Sequence
            (:then_0
              ;;[1 1 1] Planks Color
              (bind _returnvalue_13 (Rendering|Material|CreateDynamicMaterialInstance _sm_mhut_a1 1 0 "None" :!class /Script/Engine.PrimitiveComponent)))
            (:then_1
              (bind _returnvalue_14 (Rendering|Material|CreateDynamicMaterialInstance _sm_mhut_a1 2 0 "None" :!class /Script/Engine.PrimitiveComponent)))
            (:then_2
              (bind _returnvalue_15 (Rendering|Material|CreateDynamicMaterialInstance _sm_mhut_a1 4 0 "None" :!class /Script/Engine.PrimitiveComponent)))
            (:then_3
              (bind _returnvalue_16 (Rendering|Material|CreateDynamicMaterialInstance _sm_mhut_a1 5 0 "None" :!class /Script/Engine.PrimitiveComponent))))
          (Rendering|Material|SetVectorParameterValue _returnvalue_13 "Base Color" (Variables|Color|GetStairs%20Color%20B) :!class /Script/Engine.MaterialInstanceDynamic))
        (:then_2
          ;[1 1 1] Floor Color
          (bind _returnvalue_17 (Rendering|Material|CreateDynamicMaterialInstance _sm_mhut_a2 0 0 "None" :!class /Script/Engine.PrimitiveComponent))
          (Rendering|Material|SetVectorParameterValue _returnvalue_17 "Base Color" (Variables|Color|GetStairs%20Color%20A) :!class /Script/Engine.MaterialInstanceDynamic)
          (bind _returnvalue_18 (Rendering|Material|CreateDynamicMaterialInstance _sm_mhut_a2 1 0 "None" :!class /Script/Engine.PrimitiveComponent))
          (Rendering|Material|SetVectorParameterValue _returnvalue_18 "Base Color" (Variables|Color|GetStairs%20Color%20B) :!class /Script/Engine.MaterialInstanceDynamic)
          (bind _returnvalue_19 (Rendering|Material|CreateDynamicMaterialInstance (Variables|Default|GetSM_MHut_Roofs) 0 0 "None" :!class /Script/Engine.PrimitiveComponent))
          (Rendering|Material|SetVectorParameterValue _returnvalue_19 "Base Color" (Variables|Color|GetRoof%20Color) :!class /Script/Engine.MaterialInstanceDynamic))))))