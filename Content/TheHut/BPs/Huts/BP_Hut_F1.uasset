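; BP_Hut_F1 is a configurable modular hut, assembled entirely in its construction script with no active runtime logic.
; Boolean options strip the fence, pillars, floor extensions and one of two support variants, with some removals also disabling dependent floor extensions.
; A SetColor helper creates dynamic material instances to tint parts using two palette colors and a floor color.
; Forced LOD and cull distance apply to only some of the meshes.
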(event EventBeginPlay)

(event Collision|EventActorBeginOverlap
  (params (OtherActor :type Actor%20Object%20Reference)))

(event EventTick
  (params (DeltaSeconds :type Float%20%28single-precision%29)))

(fn ConstructionScript
  (bind _color_b (Variables|Color|GetColor%20B))
  (bind _floor_color (Variables|Color|GetFloor%20Color))
  (bind _sm_hutf_fence (Variables|Default|GetSM_HutF_Fence))
  (bind _sm_hutf_walls (Variables|Default|GetSM_HutF_Walls))
  (bind _color_b_2 (Variables|Color|GetColor%20B))
  (bind _color_a (Variables|Color|GetColor%20A))
  (bind _sm_hutf (Variables|Default|GetSM_HutF))
  (Utilities|FlowControl|Sequence
    (:then_0
      (if (Variables|Edit|GetFence)
        _
        (else
          (Components|DestroyComponent (Variables|Default|GetSM_HutF_Fence))))
      (if (Variables|Edit|GetSupport%20A/B)
        (Components|DestroyComponent (Variables|Default|GetSM_HutF_SupportA))
        (else
          (Components|DestroyComponent (Variables|Default|GetSM_HutF_SupportB))))
      (Utilities|FlowControl|Sequence
        (:then_0
          (if (Variables|Edit|GetPillars%20A)
            _
            (else
              (Components|DestroyComponent (Variables|Default|GetSM_HutF_PillarsA))
              (Variables|Edit|SetFloor%20Ext%20B false)))
          (if (not (Variables|Edit|GetPillars%20B))
            (Components|DestroyComponent (Variables|Default|GetSM_HutF_PillarsB))
            (Variables|Edit|SetFloor%20Ext%20C false)))
        (:then_1
          (if (Variables|Edit|GetFloor%20Ext%20A)
            _
            (else
              (Components|DestroyComponent (Variables|Default|GetSM_HutF_FloorExtA))
              (Variables|Edit|SetFloor%20Ext%20B false)))
          (if (Variables|Edit|GetFloor%20Ext%20B)
            _
            (else
              (Components|DestroyComponent (Variables|Default|GetSM_HutF_FloorExtB))))
          (if (not (Variables|Edit|GetFloor%20Ext%20C))
            (Components|DestroyComponent (Variables|Default|GetSM_HutF_FloorExtC))))))
    (:then_1
      (CallFunction|SetColor (Variables|Default|GetSM_HutF_Floor) 0 _floor_color)
      (CallFunction|SetColor (Variables|Default|GetSM_HutF_FloorExtA) 0 _floor_color)
      (CallFunction|SetColor (Variables|Default|GetSM_HutF_FloorExtB) 0 _floor_color)
      (CallFunction|SetColor (Variables|Default|GetSM_HutF_FloorExtC) 0 _floor_color)
      (CallFunction|SetColor (Variables|Default|GetSM_HutF_PillarsA) 0 _color_b)
      (CallFunction|SetColor (Variables|Default|GetSM_HutF_PillarsB) 0 _color_b)
      (CallFunction|SetColor (Variables|Default|GetSM_HutF) 0 _color_b)
      (CallFunction|SetColor _sm_hutf_fence 0 _color_b)
      (CallFunction|SetColor _sm_hutf_fence 1 (Variables|Color|GetColor%20A))
      (CallFunction|SetColor (Variables|Default|GetSM_HutF_SupportA) 0 _color_b)
      (CallFunction|SetColor (Variables|Default|GetSM_HutF_SupportB) 0 _color_b)
      (CallFunction|SetColor _sm_hutf_walls 0 _color_a)
      (CallFunction|SetColor _sm_hutf_walls 1 _color_b_2)
      (CallFunction|SetColor _sm_hutf_walls 2 _color_a)
      (CallFunction|SetColor _sm_hutf_walls 3 _color_a)
      (CallFunction|SetColor _sm_hutf_walls 5 _color_b_2)
      (CallFunction|SetColor _sm_hutf_walls 7 _color_b_2)
      (Rendering|LOD|SetForcedLodModel _sm_hutf (Variables|Edit|GetForce%20LOD))
      ;[1 0 0] If it is less than 19K, it will be discarded before LOD 3 (last LOD). 30K will have good use in open world games.
      (Class|PrimitiveComponent|SetCullDistance _sm_hutf (Variables|Edit|GetCull%20Distance)))))

(fn SetColor
  (params (Target :type Primitive%20Component%20Object%20Reference) (ElementIndex :type Integer) (Value :type Linear%20Color%20Structure))
  (bind _returnvalue (Rendering|Material|CreateDynamicMaterialInstance Target ElementIndex 0 "None" :!class /Script/Engine.PrimitiveComponent))
  (Rendering|Material|SetVectorParameterValue _returnvalue "Base Color" Value :!class /Script/Engine.MaterialInstanceDynamic))