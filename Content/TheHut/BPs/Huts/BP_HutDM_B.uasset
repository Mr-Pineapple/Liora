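; BP_HutDM_B is a configurable hut actor built from body, floor and roof static meshes, with no active gameplay logic.
; The construction script calls SetColor per material slot, creating dynamic material instances and setting "Base Color" from two main colors plus a separate roof color.
; It also applies a forced LOD and cull distance to all three meshes, with an author note on choosing cull distances for open worlds.
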(event EventBeginPlay)

(event Collision|EventActorBeginOverlap
  (params (OtherActor :type Actor%20Object%20Reference)))

(event EventTick
  (params (DeltaSeconds :type Float%20%28single-precision%29)))

(fn ConstructionScript
  (bind _sm_hutd (Variables|Default|GetSM_HutD))
  (bind _sm_hutd_2 (Variables|Default|GetSM_HutD))
  (bind _color_a (Variables|Color|GetColor%20A))
  (bind _color_b (Variables|Color|GetColor%20B))
  (bind _sm_hutd_floor (Variables|Default|GetSM_HutD_Floor))
  (bind _color_b_2 (Variables|Color|GetColor%20B))
  (bind _sm_hutd_roof (Variables|Default|GetSM_HutD_Roof))
  (Utilities|FlowControl|Sequence
    (:then_0
      ;[1 1 1] Hut Color
      (CallFunction|SetColor _sm_hutd_2 0 _color_a)
      (CallFunction|SetColor _sm_hutd_2 1 _color_b)
      (CallFunction|SetColor _sm_hutd_2 3 _color_b)
      (CallFunction|SetColor _sm_hutd_2 4 _color_a)
      (CallFunction|SetColor _sm_hutd_2 5 _color_a)
      (CallFunction|SetColor _sm_hutd_2 6 _color_a)
      (CallFunction|SetColor _sm_hutd_2 7 _color_b))
    (:then_1
      (CallFunction|SetColor _sm_hutd_floor 0 (Variables|Color|GetColor%20B))
      (CallFunction|SetColor _sm_hutd_floor 1 (Variables|Color|GetColor%20A)))
    (:then_2
      (CallFunction|SetColor _sm_hutd_roof 0 (Variables|Color|GetColor%20A))
      (CallFunction|SetColor _sm_hutd_roof 1 _color_b_2)
      (CallFunction|SetColor _sm_hutd_roof 2 (Variables|Color|GetRoof%20Color))
      (CallFunction|SetColor _sm_hutd_roof 3 _color_b_2))
    (:then_3
      (Rendering|LOD|SetForcedLodModel _sm_hutd (Variables|Edit|GetForce%20LOD))
      ;[1 0 0] If it is less than 19K, it will be discarded before LOD 3 (last LOD). 30K will have good use in open world games.
      (Class|PrimitiveComponent|SetCullDistance _sm_hutd (Variables|Edit|GetCull%20Distance)))))

(fn SetColor
  (params (SM%20Target%20 :type Primitive%20Component%20Object%20Reference) (Index%20MAT :type Integer) (Color :type Linear%20Color%20Structure))
  (bind _returnvalue (Rendering|Material|CreateDynamicMaterialInstance SM%20Target%20 Index%20MAT 0 "None" :!class /Script/Engine.PrimitiveComponent))
  (Rendering|Material|SetVectorParameterValue _returnvalue "Base Color" Color :!class /Script/Engine.MaterialInstanceDynamic))