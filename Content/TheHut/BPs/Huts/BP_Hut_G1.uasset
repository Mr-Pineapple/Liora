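; BP_Hut_G1 is a configurable hut actor built from static mesh parts for body, roof, floor, ceiling and walls.
; Its construction script removes the ceiling and walls when their toggles are off, then applies forced LOD and cull distance to the parts.
; A SetColor helper creates dynamic material instances to tint the body, roof, ceiling and floor, with body and roof sharing one color.
; The event graph holds no active logic.
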(event EventBeginPlay)

(event Collision|EventActorBeginOverlap
  (params (OtherActor :type Actor%20Object%20Reference)))

(event EventTick
  (params (DeltaSeconds :type Float%20%28single-precision%29)))

(fn ConstructionScript
  (bind _sm_hutg (Variables|Default|GetSM_HutG))
  (Utilities|FlowControl|Sequence
    (:then_0
      (if (Variables|Edit|GetCeiling)
        _
        (else
          (Components|DestroyComponent (Variables|Default|GetSM_HutG_Ceiling))))
      (if (not (Variables|Edit|GetWalls))
        (Components|DestroyComponent (Variables|Default|GetSM_HutG_Walls))))
    (:then_1
      (CallFunction|SetColor (Variables|Default|GetSM_HutG) 0 (Variables|Color|GetColor%20B))
      (CallFunction|SetColor (Variables|Default|GetSM_HutG_Ceiling) 0 (Variables|Color|GetCeiling%20Color))
      (CallFunction|SetColor (Variables|Default|GetSM_HutG_Floor) 0 (Variables|Color|GetFloor%20Color))
      (CallFunction|SetColor (Variables|Default|GetSM_HutG_Roof) 0 (Variables|Color|GetColor%20B))
      (Rendering|LOD|SetForcedLodModel _sm_hutg (Variables|Edit|GetForce%20LOD))
      ;[1 0 0] If it is less than 19K, it will be discarded before LOD 3 (last LOD). 30K will have good use in open world games.
      (Class|PrimitiveComponent|SetCullDistance _sm_hutg (Variables|Edit|GetCull%20Distance)))))

(fn SetColor
  (params (Target :type Primitive%20Component%20Object%20Reference) (ElementIndex :type Integer) (Value :type Linear%20Color%20Structure))
  (bind _returnvalue (Rendering|Material|CreateDynamicMaterialInstance Target ElementIndex 0 "None" :!class /Script/Engine.PrimitiveComponent))
  (Rendering|Material|SetVectorParameterValue _returnvalue "Base Color" Value :!class /Script/Engine.MaterialInstanceDynamic))