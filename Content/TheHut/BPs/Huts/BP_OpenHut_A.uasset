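; BP_OpenHut_A is a configurable open hut building made of body, roof and pillar foundation meshes, set up entirely in the Construction Script.
; Options switch the scene's X scale for the roof variant, remove the pillar foundation, and apply a forced LOD and cull distance to the meshes.
; A SetColor helper creates dynamic material instances per material slot, tinting the parts with two exposed colors through the "Base Color" parameter.
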(event EventBeginPlay)

(event Collision|EventActorBeginOverlap
  (params (OtherActor :type Actor%20Object%20Reference)))

(event EventTick
  (params (DeltaSeconds :type Float%20%28single-precision%29)))

(fn ConstructionScript
  (bind _color_a (Variables|Color|GetColor%20A))
  (bind _color_b (Variables|Color|GetColor%20B))
  (bind _sm_hutb (Variables|Default|GetSM_HutB))
  (bind _scene (Variables|Default|GetScene))
  (bind _sm_hutb_2 (Variables|Default|GetSM_HutB))
  (bind _sm_hutpillar (Variables|Default|GetSM_HutPillar))
  (bind _sm_hutaroof (Variables|Default|GetSM_HutARoof))
  (Utilities|FlowControl|Sequence
    (:then_0
      (if (Variables|Edit|GetRoof%20A/B)
        (Transformation|SetRelativeScale3D _scene "1.000000,1.000000,1.000000")
        (else
          (Transformation|SetRelativeScale3D _scene "1.250000,1.000000,1.000000")))
      (if (Variables|Edit|GetPillarFundation)
        _
        (else
          (Components|DestroyComponent (Variables|Default|GetSM_HutPillar))))
      (Rendering|LOD|SetForcedLodModel _sm_hutb (Variables|Edit|GetForce%20LOD))
      ;[1 0 0] If it is less than 19K, it will be discarded before LOD 3 (last LOD). 30K will have good use in open world games.
      (Class|PrimitiveComponent|SetCullDistance _sm_hutb (Variables|Edit|GetCull%20Distance)))
    (:then_1
      (CallFunction|SetColor _sm_hutb_2 0 _color_a)
      (CallFunction|SetColor _sm_hutb_2 1 _color_a)
      (CallFunction|SetColor _sm_hutb_2 2 _color_a)
      (CallFunction|SetColor _sm_hutb_2 3 _color_a)
      (CallFunction|SetColor _sm_hutb_2 4 _color_b)
      (CallFunction|SetColor _sm_hutb_2 5 _color_b)
      (CallFunction|SetColor _sm_hutpillar 0 _color_b)
      (CallFunction|SetColor _sm_hutpillar 1 _color_b)
      (CallFunction|SetColor _sm_hutaroof 0 _color_b)
      (CallFunction|SetColor _sm_hutaroof 1 _color_b)
      (CallFunction|SetColor _sm_hutaroof 4 _color_b)
      (CallFunction|SetColor _sm_hutaroof 2 _color_a))))

(fn SetColor
  (params (Target :type Primitive%20Component%20Object%20Reference) (ElementIndex :type Integer) (Value :type Linear%20Color%20Structure))
  (bind _returnvalue (Rendering|Material|CreateDynamicMaterialInstance Target ElementIndex 0 "None" :!class /Script/Engine.PrimitiveComponent))
  (Rendering|Material|SetVectorParameterValue _returnvalue "Base Color" Value :!class /Script/Engine.MaterialInstanceDynamic))