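; BP_Planks_A1 is a plank set actor that randomizes its look at construction, with no active runtime logic.
; The Construction Script gives each of fifteen plank components a random mesh from NewSMs, within the RandomMin to RandomMax index range.
; Cull distance and forced LOD are set inside that loop but only ever target SMPlankA1.
; The script also resets the Update flag to false on every run.
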(event EventBeginPlay)

(event Collision|EventActorBeginOverlap
  (params (OtherActor :type Actor%20Object%20Reference)))

(event EventTick
  (params (DeltaSeconds :type Float%20%28single-precision%29)))

(fn ConstructionScript
  (bind _sm_plank_a1 (Variables|Default|GetSM_Plank_A1))
  (Variables|Mesh|SetUpdate false)
  (for _array_element (Utilities|Array|MakeArray _sm_plank_a1 (Variables|Default|GetSM_Plank_A2) (Variables|Default|GetSM_Plank_A3) (Variables|Default|GetSM_Plank_A4) (Variables|Default|GetSM_Plank_A5) (Variables|Default|GetSM_Plank_A6) (Variables|Default|GetSM_Plank_A7) (Variables|Default|GetSM_Plank_A8) (Variables|Default|GetSM_Plank_A9) (Variables|Default|GetSM_Plank_A10) (Variables|Default|GetSM_Plank_A11) (Variables|Default|GetSM_Plank_A12) (Variables|Default|GetSM_Plank_A13) (Variables|Default|GetSM_Plank_A14) (Variables|Default|GetSM_Plank_A15))
    (Components|StaticMesh|SetStaticMesh _array_element (Utilities|Array|Get(acopy) (Variables|Mesh|GetNew%20SMs) (Math|Random|RandomIntegerinRange (Variables|Mesh|GetRandom%20Min) (Variables|Mesh|GetRandom%20Max))))
    (Class|PrimitiveComponent|SetCullDistance _sm_plank_a1 (Variables|Mesh|GetCull%20Distance))
    (Rendering|LOD|SetForcedLodModel _sm_plank_a1 (Variables|Mesh|GetForce%20LOD%20Models))))