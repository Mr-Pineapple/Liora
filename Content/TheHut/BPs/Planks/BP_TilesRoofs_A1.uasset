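; BP_TilesRoofs_A1 is a construction-script tool that procedurally builds a row of roof tile or plank meshes for the hut.
; It adds a static mesh component per instance, spaced along local Z from a base transform, with random pitch and X scale for variation.
; Each piece gets a random mesh from an array index range, plus a cull distance and forced LOD.
; The event graph is unused.
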(event EventBeginPlay)

(event Collision|EventActorBeginOverlap
  (params (OtherActor :type Actor%20Object%20Reference)))

(event EventTick
  (params (DeltaSeconds :type Float%20%28single-precision%29)))

(fn ConstructionScript
  (bind _planks_location (Variables|Default|GetPlanks%20Location))
  (bind (_location _rotation _scale) (Math|Transform|BreakTransform _planks_location))
  (Variables|Mesh|SetUpdate false)
  (for _index (range 0 (- (Variables|Default|GetInstances) 1))
    (Variables|Default|SetIndex _index)
    (bind _returnvalue (AddComponent|AddStaticMeshComponent false (Math|Transform|MakeTransform (Math|Vector|MakeVector (.x _location) (.y _location) (+ (* (Variables|Default|GetIndex) (Variables|Default|GetDistance%20by%20SMs)) (.z _location))) (Math|Rotator|MakeRotator (.roll _rotation) (+ (.pitch _rotation) (Math|Random|RandomFloatinRange (Variables|Default|GetRotation%20Min) (Variables|Default|GetRotation%20Max))) (.yaw _rotation)) (Math|Vector|MakeVector (Math|Random|RandomFloatinRange (Variables|Default|GetScale%20Min) (Variables|Default|GetScale%20Max)) (.y _scale) (Variables|Default|GetScaleZ)))))
    (Components|StaticMesh|SetStaticMesh _returnvalue (Utilities|Array|Get(acopy) (Variables|Mesh|GetNew%20SMs) (Math|Random|RandomIntegerinRange (Variables|Default|GetWall%20-%20Random%20Min) (Variables|Default|GetWall%20-%20Random%20Max))))
    (Class|PrimitiveComponent|SetCullDistance _returnvalue (Variables|Mesh|GetCull%20Distance))
    (Rendering|LOD|SetForcedLodModel _returnvalue (Variables|Mesh|GetForce%20LOD%20Models))))