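; BP_Stairs_B1 is a stair actor for TheHut, built from plank static mesh components.
; Its Construction Script gives each listed plank a random mesh from the PlanksSMs array, within a configurable index range, for visual variation.
; The same loop applies a shared cull distance and forced LOD to each plank.
; The event graph holds no logic.
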(event EventBeginPlay)

(event Collision|EventActorBeginOverlap
  (params (OtherActor :type Actor%20Object%20Reference)))

(event EventTick
  (params (DeltaSeconds :type Float%20%28single-precision%29)))

(fn ConstructionScript
  (for _array_element (Utilities|Array|MakeArray (Variables|Default|GetSM_Plank_A1) (Variables|Default|GetSM_Plank_A10) (Variables|Default|GetSM_Plank_A11) (Variables|Default|GetSM_Plank_A12) (Variables|Default|GetSM_Plank_A12_12A) (Variables|Default|GetSM_Plank_A12_12B) (Variables|Default|GetSM_Plank_B6) (Variables|Default|GetSM_Plank_B1))
    (Components|StaticMesh|SetStaticMesh _array_element (Utilities|Array|Get(acopy) (Variables|Default|GetPlanks%20SMs) (Math|Random|RandomIntegerinRange (Variables|Default|GetSM%20-%20Random%20Min) (Variables|Default|GetSM%20-%20Random%20Max))))
    (Class|PrimitiveComponent|SetCullDistance _array_element (Variables|Default|GetCull%20Distance))
    (Rendering|LOD|SetForcedLodModel _array_element (Variables|Default|GetForce%20LOD%20Models))))