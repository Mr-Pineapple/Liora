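; Modular roof building actor for the Hut set that assembles a roof procedurally in its Construction Script.
; Transform arrays place beams and rafters, plus optional tiles, wall pieces and fascia boards, as static mesh components with meshes picked at random from per-part lists.
; Optional pillars reuse the beam transforms for sideways position and rotation, with adjustable slide and height, while tiles get an adjustable Z scale.
; The event graph is unused.
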(event EventBeginPlay)

(event Collision|EventActorBeginOverlap
  (params (OtherActor :type Actor%20Object%20Reference)))

(event EventTick
  (params (DeltaSeconds :type Float%20%28single-precision%29)))

(fn ConstructionScript
  (Variables|Beam|SetUpdate%20All false)
  (Utilities|FlowControl|Sequence
    (:then_0
      (for _array_element (Variables|Beam|GetBeam%20Location)
        (bind _returnvalue (AddComponent|AddStaticMeshComponent false _array_element))
        (Components|StaticMesh|SetStaticMesh _returnvalue (Utilities|Array|Get(acopy) (Variables|Beam|GetBeam%20-%20New%20SMs) (Math|Random|RandomIntegerinRange (Variables|Beam|GetBeam%20-%20Random%20Min) (Variables|Beam|GetBeam%20-%20Random%20Max))))))
    (:then_1
      (for _array_element_2 (Variables|Rafter|GetRafter%20Location)
        (bind _returnvalue_2 (AddComponent|AddStaticMeshComponent false _array_element_2))
        (Components|StaticMesh|SetStaticMesh _returnvalue_2 (Utilities|Array|Get(acopy) (Variables|Rafter|GetRafter%20-%20New%20SMs) (Math|Random|RandomIntegerinRange (Variables|Rafter|GetRafter%20-%20Random%20Min) (Variables|Rafter|GetRafter%20-%20Random%20Max))))))
    (:then_2
      (if (Variables|Tiles|GetHave%20Tiles)
        (for _array_element_3 (Variables|Tiles|GetTiles%20Location)
          (bind _returnvalue_3 (AddComponent|AddStaticMeshComponent false (Math|Transform|MakeTransform (.Location (Math|Transform|BreakTransform _array_element_3)) (.Rotation (Math|Transform|BreakTransform _array_element_3)) (Math|Vector|MakeVector (.x (.Scale (Math|Transform|BreakTransform _array_element_3))) (.y (.Scale (Math|Transform|BreakTransform _array_element_3))) (* (.z (.Scale (Math|Transform|BreakTransform _array_element_3))) (Variables|Tiles|GetLeight%20Tiles%20%28Scale%29))))))
          (Components|StaticMesh|SetStaticMesh _returnvalue_3 (Utilities|Array|Get(acopy) (Variables|Tiles|GetTiles%20-%20New%20SMs) (Math|Random|RandomIntegerinRange (Variables|Tiles|GetTiles%20-%20Random%20Min) (Variables|Tiles|GetTiles%20-%20Random%20Max)))))))
    (:then_3
      (if (Variables|Pillars|GetHave%20Pillar)
        (for _array_element_4 (Variables|Beam|GetBeam%20Location)
          (bind _returnvalue_4 (AddComponent|AddStaticMeshComponent false (Math|Transform|MakeTransform (Math|Vector|MakeVector (* (+ (Variables|Pillars|GetSlide%20Pillars%20%20%28Location%29) 1.0) -1.0) (+ (.y (.Location (Math|Transform|BreakTransform _array_element_4))) 2.0) -19.0) (.Rotation (Math|Transform|BreakTransform _array_element_4)) (Math|Vector|MakeVector 1.0 1.2 (Variables|Pillars|GetHeght%20Pillars%20%28Scale%20Z%29)))))
          (Components|StaticMesh|SetStaticMesh _returnvalue_4 (Utilities|Array|Get(acopy) (Variables|Pillars|GetPillars%20-%20SMs) (Math|Random|RandomIntegerinRange 0 0))))))
    (:then_4
      (if (Variables|Walls|GetHave%20Walls)
        (for _array_element_5 (Variables|Walls|GetWallRoof)
          (bind _returnvalue_5 (AddComponent|AddStaticMeshComponent false _array_element_5))
          (Components|StaticMesh|SetStaticMesh _returnvalue_5 (Utilities|Array|Get(acopy) (Variables|Walls|GetWallRoof%20-%20SMs) (Math|Random|RandomIntegerinRange 0 2))))))
    (:then_5
      (if (Variables|FasciaBoard|GetHave%20FasciaBoard)
        (for _array_element_6 (Variables|FasciaBoard|GetFasciaBoard)
          (bind _returnvalue_6 (AddComponent|AddStaticMeshComponent false _array_element_6))
          (Components|StaticMesh|SetStaticMesh _returnvalue_6 (Utilities|Array|Get(acopy) (Variables|FasciaBoard|GetFasciaBoard%20-%20SMs) (Math|Random|RandomIntegerinRange 0 0))))))))