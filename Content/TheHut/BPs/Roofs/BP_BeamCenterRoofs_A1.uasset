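; Procedural roof beam builder that lays out repeated centre beams for a roof structure in its construction script.
; For each instance it adds optional A, B and C static mesh components, spaced along Y, with Z scale driven by structure length or pillar height.
; The optional last beam is re-added at one fixed offset on every iteration.
; Random plank mesh, cull distance and forced LOD nodes are disconnected and never run.
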(event EventBeginPlay)

(event Collision|EventActorBeginOverlap
  (params (OtherActor :type Actor%20Object%20Reference)))

(event EventTick
  (params (DeltaSeconds :type Float%20%28single-precision%29)))

(fn ConstructionScript
  (bind _beam_location_a (Variables|Mesh|GetBeam%20Location%20A))
  (bind _beam_location_c (Variables|Mesh|GetBeam%20Location%20C))
  (bind _leight_structure (Variables|Mesh|GetLeight%20Structure))
  (bind _last_beam_location (Variables|Mesh|GetLast%20Beam%20location))
  (bind _beam_location_b (Variables|Mesh|GetBeam%20Location%20B))
  (bind (_location _rotation _scale) (Math|Transform|BreakTransform _beam_location_a))
  (bind (_location_2 _rotation_2 _scale_2) (Math|Transform|BreakTransform _last_beam_location))
  (bind (_location_3 _rotation_3 _scale_3) (Math|Transform|BreakTransform _beam_location_b))
  (bind (_location_4 _rotation_4 _scale_4) (Math|Transform|BreakTransform _beam_location_c))
  (bind _returnvalue (+ _leight_structure 0.0))
  (Variables|Mesh|SetUpdate false)
  (for _index (range 0 (- (Variables|Mesh|GetInstances) 1))
    (Variables|Default|SetIndex _index)
    (if (Variables|Mesh|GetBeam%20B)
      (bind _returnvalue_2 (AddComponent|AddStaticMeshComponent false (Math|Transform|MakeTransform (Math|Vector|MakeVector (.x _location_3) (+ (* (Variables|Default|GetIndex) (Variables|Mesh|GetDistance%20by%20SMs)) (.y _location_3)) (+ (Variables|Mesh|GetHeght%20Beam) 0.0)) (Math|Rotator|MakeRotator (.roll _rotation_3) (.pitch _rotation_3) (.yaw _rotation_3)) (Math|Vector|MakeVector (.x _scale_3) (.y _scale_3) _returnvalue)))))
    (if (Variables|Mesh|GetBeam%20A)
      (AddComponent|AddStaticMeshComponent false (Math|Transform|MakeTransform (Math|Vector|MakeVector (.x _location) (+ (* (Variables|Default|GetIndex) (Variables|Mesh|GetDistance%20by%20SMs)) (.y _location)) (.z _location)) (Math|Rotator|MakeRotator (.roll _rotation) (.pitch _rotation) (.yaw _rotation)) (Math|Vector|MakeVector (.x _scale) (.y _scale) _returnvalue))))
    (if (Variables|Mesh|GetBeam%20C)
      (AddComponent|AddStaticMeshComponent false (Math|Transform|MakeTransform (Math|Vector|MakeVector (.x _location_4) (+ (* (Variables|Default|GetIndex) (Variables|Mesh|GetDistance%20by%20SMs)) (.y _location_4)) (.z _location_4)) (Math|Rotator|MakeRotator (.roll _rotation_4) (.pitch _rotation_4) (.yaw _rotation_4)) (Math|Vector|MakeVector (.x _scale_4) (.y _scale_4) (+ (Variables|Mesh|GetHeight%20Pillar) 0.0)))))
    (if (Variables|Mesh|GetLast%20Beam)
      (AddComponent|AddStaticMeshComponent false (Math|Transform|MakeTransform (Math|Vector|MakeVector (.x _location_2) (+ (Variables|Mesh|GetDistance%20by%20SMs) (.y _location_2)) (.z _location_2)) (Math|Rotator|MakeRotator (.roll _rotation_2) (.pitch _rotation_2) (.yaw _rotation_2)) (Math|Vector|MakeVector (.x _scale_2) (.y _scale_2) (+ (Variables|Mesh|GetHeight%20Pillar) 0.0)))))))