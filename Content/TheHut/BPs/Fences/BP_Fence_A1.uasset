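; BP_Fence_A1 is a procedural fence actor that builds a row of fence meshes in its construction script, with no active event logic.
; Each instance gets its own static mesh component, spaced along local Y by a set distance, with a random plank mesh from an array range.
; An optional end beam is placed at the row's far end, added inside the same loop.
; Cull distance and forced LOD are applied to the spawned components.
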(event EventBeginPlay)

(event Collision|EventActorBeginOverlap
  (params (OtherActor :type Actor%20Object%20Reference)))

(event EventTick
  (params (DeltaSeconds :type Float%20%28single-precision%29)))

(fn ConstructionScript
  (Variables|Mesh|SetUpdate false)
  (for _index (range 0 (- (Variables|Mesh|GetInstances) 1))
    (Variables|Mesh|SetIndex _index)
    (bind _returnvalue (AddComponent|AddStaticMeshComponent false (|LocationOfFences)))
    (if (Variables|Mesh|GetLast%20Beam)
      (bind _returnvalue_2 (AddComponent|AddStaticMeshComponent false (|LOcationofLastBeam))))
    (Components|StaticMesh|SetStaticMesh _returnvalue (Utilities|Array|Get(acopy) (Variables|Mesh|GetPlanks%20SMs) (Math|Random|RandomIntegerinRange (Variables|Mesh|GetSM%20-%20Random%20Min) (Variables|Mesh|GetSM%20-%20Random%20Max))))
    (Class|PrimitiveComponent|SetCullDistance _returnvalue (Variables|Mesh|GetCull%20Distance))
    (Rendering|LOD|SetForcedLodModel _returnvalue (Variables|Mesh|GetForce%20LOD%20Models))))