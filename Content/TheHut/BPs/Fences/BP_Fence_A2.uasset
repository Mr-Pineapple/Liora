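; BP_Fence_A2 is a construction-script fence builder that lays out a row of plank meshes for level dressing.
; It adds one static mesh component per instance, stepped along local Y by a fixed spacing from an editable base transform.
; Each component takes a random mesh from an index range of the plank array, plus shared cull distance and forced LOD settings.
; The event graph holds no active logic.
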(event EventBeginPlay)

(event Collision|EventActorBeginOverlap
  (params (OtherActor :type Actor%20Object%20Reference)))

(event EventTick
  (params (DeltaSeconds :type Float%20%28single-precision%29)))

(fn ConstructionScript
  (bind _fence_location (Variables|Mesh|GetFence%20Location))
  (bind (_location _rotation _scale) (Math|Transform|BreakTransform _fence_location))
  (Variables|Mesh|SetUpdate false)
  (for _index (range 0 (- (Variables|Mesh|GetInstances) 1))
    (Variables|Mesh|SetIndex _index)
    (bind _returnvalue (AddComponent|AddStaticMeshComponent false (Math|Transform|MakeTransform (Math|Vector|MakeVector (.x _location) (+ (* (Variables|Mesh|GetIndex) (Variables|Mesh|GetDistance%20by%20SMs)) (.y _location)) (.z _location)) (Math|Rotator|MakeRotator (.roll _rotation) (.pitch _rotation) (.yaw _rotation)) (Math|Vector|MakeVector (.x _scale) (.y _scale) (.z _scale)))))
    (Components|StaticMesh|SetStaticMesh _returnvalue (Utilities|Array|Get(acopy) (Variables|Mesh|GetPlanks%20SMs) (Math|Random|RandomIntegerinRange (Variables|Mesh|GetSM%20-%20Random%20Min) (Variables|Mesh|GetSM%20-%20Random%20Max))))
    (Class|PrimitiveComponent|SetCullDistance _returnvalue (Variables|Mesh|GetCull%20Distance))
    (Rendering|LOD|SetForcedLodModel _returnvalue (Variables|Mesh|GetForce%20LOD%20Models))))